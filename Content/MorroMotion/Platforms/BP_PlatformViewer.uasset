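; BP_PlatformViewer is a view-target actor that pans steadily through the level, apparently for viewing platforms.
; On BeginPlay it becomes the first player controller's view target, adds the WBP_Controls widget to the viewport and hides the mesh of every DefaultPawn.
; Each Tick it moves itself along the Y axis by PanSpeed, without delta-time scaling, so pan speed depends on frame rate.
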(event EventTick
  (params (DeltaSeconds :type Float%20%28single-precision%29))
  (Transformation|SetActorLocation (+ (Transformation|GetActorLocation) (Math|Vector|MakeVector 0.0 (Variables|Default|GetPan_Speed) 0.0)) false false))

(event EventBeginPlay
  (Game|Player|SetViewTargetwithBlend (Game|GetPlayerController 0) self 0.0 "VTBlend_Linear" 0.0 false)
  (bind _returnvalue (UserInterface|CreateWidget "/Game/MorroMotion/Platforms/WBP_Controls.WBP_Controls_C"))
  (UserInterface|Viewport|AddtoViewport _returnvalue 0)
  (|Hide_Default_Pawn))

(fn ConstructionScript)