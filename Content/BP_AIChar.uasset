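; AI character Blueprint that turns body-pose landmark vectors into IK target locations.
; SkeletalDataUpdate draws landmarks as debug boxes, then sets targets: axis-swapped via CoordinateTransfer for head, hands and feet, offset by mesh location for shoulders, elbows, hips and knees.
; Socket connection, data receive and the looping update timer are disconnected, so BeginPlay only prints a TestFunc result.
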(event Custom|Skeletal%20data%20update
  (bind _landmarkvectors (Variables|Default|GetLandmarkVectors))
  (bind _mesh (Variables|Character|GetMesh))
  (bind _returnvalue (Transformation|GetWorldLocation _mesh))
  ;[1 1 1] Bone Update (showing in level)
  ;;[1 1 1] Debug_Drawing_Landmark_Dot
  (for (_array_element _array_index) _landmarkvectors
    (if (== _array_index 16)
      (Rendering|Debug|DrawDebugBox (+ (Math|Vector|MakeVector (.x _returnvalue) (.y _returnvalue) (.z _returnvalue)) (Math|Vector|MakeVector (.x (* _array_element 1.0)) (.y (* _array_element 1.0)) (+ (.z (* _array_element 1.0)) 0.0))) "2.000000,2.000000,2.000000" "(R=0.000000,G=1.000000,B=0.470318,A=1.000000)" "0, 0, 0" 0.1 2.0)
      (else
        (Rendering|Debug|DrawDebugBox (+ (Math|Vector|MakeVector (.x _returnvalue) (.y _returnvalue) (.z _returnvalue)) (Math|Vector|MakeVector (.x (* _array_element 1.0)) (.y (* _array_element 1.0)) (+ (.z (* _array_element 1.0)) 0.0))) "2.000000,2.000000,2.000000" "(R=1.000000,G=0.000000,B=0.000000,A=1.000000)" "0, 0, 0" 0.3 2.0))))
  ;;[1 1 1] for IK
  (Variables|Default|SetLoc_Head (CallFunction|CoordinateTransfer (Utilities|Array|Get(acopy) _landmarkvectors 10)))
  (Variables|Default|SetLoc_LeftShoulder (+ (Utilities|Array|Get(acopy) _landmarkvectors 11) (Transformation|GetWorldLocation (Variables|Character|GetMesh))))
  (Variables|Default|SetLoc_RightShoulder (+ (Utilities|Array|Get(acopy) _landmarkvectors 12) (Transformation|GetWorldLocation (Variables|Character|GetMesh))))
  (Variables|Default|SetLoc_LeftElbow (+ (Utilities|Array|Get(acopy) _landmarkvectors 13) (Transformation|GetWorldLocation (Variables|Character|GetMesh))))
  (Variables|Default|SetLoc_RightElbow (+ (Utilities|Array|Get(acopy) _landmarkvectors 14) (Transformation|GetWorldLocation (Variables|Character|GetMesh))))
  (Variables|Default|SetLoc_LeftHand (CallFunction|CoordinateTransfer (Utilities|Array|Get(acopy) _landmarkvectors 15)))
  (Variables|Default|SetLoc_RightHand (CallFunction|CoordinateTransfer (Utilities|Array|Get(acopy) _landmarkvectors 16)))
  (Variables|Default|SetLoc_LeftHip (+ (Utilities|Array|Get(acopy) _landmarkvectors 23) (Transformation|GetWorldLocation (Variables|Character|GetMesh))))
  (Variables|Default|SetLoc_RightHip (+ (Utilities|Array|Get(acopy) _landmarkvectors 24) (Transformation|GetWorldLocation (Variables|Character|GetMesh))))
  (Variables|Default|SetLoc_LeftKnee (+ (Utilities|Array|Get(acopy) _landmarkvectors 25) (Transformation|GetWorldLocation (Variables|Character|GetMesh))))
  (Variables|Default|SetLocation_RightKnee (+ (Utilities|Array|Get(acopy) _landmarkvectors 26) (Transformation|GetWorldLocation (Variables|Character|GetMesh))))
  (Variables|Default|SetLoc_LeftFoot (CallFunction|CoordinateTransfer (Utilities|Array|Get(acopy) _landmarkvectors 27)))
  (Variables|Default|SetLoc_RightFoot (CallFunction|CoordinateTransfer (Utilities|Array|Get(acopy) _landmarkvectors 28))))

(event EventBeginPlay
  (bind _returnvalue (Class|MyCharacter|TestFunc (Variables|Default|GetAnyVectorA) (Variables|Default|GetAnyVectorB)))
  (Development|PrintString (Utilities|String|ToString(Float) _returnvalue) true true "(R=1.000000,G=0.025803,B=0.000000,A=1.000000)" 15.0))

(event Collision|EventActorBeginOverlap
  (params (OtherActor :type Actor%20Object%20Reference)))

(event EventTick
  (params (DeltaSeconds :type Float%20%28single-precision%29))
  ;[1 1 1] Recieve data
)

(fn ConstructionScript)

(fn CoordinateTransfer
  (params (InputVector :type Vector))
  (bind (_x _y _z) (Math|Vector|BreakVector InputVector))
  (return (Math|Vector|MakeVector _y (* _x -1.0) _z)))